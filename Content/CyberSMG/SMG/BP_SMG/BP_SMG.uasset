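; BP_SMG is a submachine gun Blueprint with optional full magazine, aim sight and silencer parts.
; The Construction Script sets each part's visibility from boolean variables, with VisibleAim driving the sight mesh and its glass.
; The sight's FGlass mesh is set twice, ending visible only when both VisibleAim and HideAimFGlass are true, despite that flag's name.
; The event graph holds only empty events, so no firing or gameplay logic exists here.
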(event `self.ReceiveTick`
  (params (DeltaSeconds :type "Float (single-precision)")))

(fn `UserConstructionScript`
  (bind _visibleaim_ (`self.VisibleAim?`))
  (`SceneComponent.SetVisibility` (`self.SK_FullMag`) (`self.VisibleFullMag`) false)
  (`SceneComponent.SetVisibility` (`self.SK_Aim`) _visibleaim_ false)
  (`SceneComponent.SetVisibility` (`self.SM_GlassAim`) _visibleaim_ false)
  (`SceneComponent.SetVisibility` (`self.SM_FGlassAim`) _visibleaim_ false)
  (`SceneComponent.SetVisibility` (`self.SM_FGlassAim`) (and _visibleaim_ (`self.HideAimFGlass?`)) false)
  (`SceneComponent.SetVisibility` (`self.SM_Silences`) (`self.VisibleSilence?`) false))