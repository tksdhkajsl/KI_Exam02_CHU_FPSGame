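; BP_EquipWeaponMaster is a weapon Blueprint that, by its name, serves as the master class for equipped weapons.
; Its construction script looks up the WeaponData row handle and copies that row's identity, combat stats, fire settings and pickup/equip references into variables.
; The SetFirMode event overwrites the current fire mode, while the Fire event is an empty stub with no firing logic in this graph.
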(event `/Game/MainContents/Interfaces/BPI_Fire.Fire`
  (params (IsFiring :type Boolean)))

(event `/Game/MainContents/Interfaces/BPI_EquipWeaponInterface.SetFirMode`
  (params (FireMode :type "/Game/MainContents/Weapons/E_FireMode Enum" :default "NewEnumerator0"))
  (set `self.FireMode` FireMode))

(fn `UserConstructionScript`
  (bind (_datatable _rowname) (break `DataTableRowHandle` (`self.WeaponData`)))
  (bind _returnvalue (`|GetDataTableRow` _datatable _rowname)
    (:`then`
      (bind (_weaponname _weapontype _damage _magazinesize _pickupweapon _equipweapon _firemode _firerate) (break `/Game/MainContents/Weapons/S_Weapon` _returnvalue))
      (set `self.Weapon Name` _weaponname)
      (set `self.Weapon Type` _weapontype)
      (set `self.Damage` _damage)
      (set `self.Magazine Size` _magazinesize)
      (set `self.Pickup Weapon` _pickupweapon)
      (set `self.Equip Weapon` _equipweapon)
      (set `self.FireMode` _firemode)
      (set `self.FireRate` _firerate))))