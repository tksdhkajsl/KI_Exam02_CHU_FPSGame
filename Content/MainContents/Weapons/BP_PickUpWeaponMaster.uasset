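; Base pickup weapon actor that hands a weapon to a player character and then removes itself from the level.
; A sphere overlap shows the pickup's widget and end overlap hides it, with no check on which actor overlaps.
; The PickUp event looks up the WeaponData table row, passes its EquipWeapon to the character's PickUpWeapon, and destroys the actor only when the row is found.
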(event `/Game/MainContents/Interfaces/BPI_Interact.PickUp`
  (params (PlayerCharactor :type "/Game/MainContents/Charactor/Player/BP_Player Object Reference"))
  (bind (_datatable _rowname) (break `DataTableRowHandle` (`self.WeaponData`)))
  (bind _returnvalue (`|GetDataTableRow` _datatable _rowname)
    (:`then`
      (`/Game/MainContents/Charactor/Player/BP_Player.PickUpWeapon` PlayerCharactor (`.EquipWeapon_18_1FC903954A3ED488378C6689EDD02F42` (break `/Game/MainContents/Weapons/S_Weapon` _returnvalue)))
      (`self.K2_DestroyActor`))))

(event `self.Sphere.OnComponentBeginOverlap`
  (params (OverlappedComponent :type "PrimitiveComponent Object Reference") (OtherActor :type "Actor Object Reference") (OtherComp :type "PrimitiveComponent Object Reference") (OtherBodyIndex :type Integer) (bFromSweep :type Boolean) (SweepResult :type "HitResult Structure (by ref)"))
  (`SceneComponent.SetVisibility` (`self.Widget`) true false))

(event `self.Sphere.OnComponentEndOverlap`
  (params (OverlappedComponent :type "PrimitiveComponent Object Reference") (OtherActor :type "Actor Object Reference") (OtherComp :type "PrimitiveComponent Object Reference") (OtherBodyIndex :type Integer))
  (`SceneComponent.SetVisibility` (`self.Widget`) false false))

(fn `UserConstructionScript`)