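; BPC_StatSystem is a stat component that tracks health and death state for its owner.
; On BeginPlay it sets CurrentHealth to MaxHealth; IncreaseHealth adds points and caps the result at MaxHealth.
; DecreaseHealth computes DamagePoint minus CurrentHealth (operands reversed from usual damage subtraction), then at zero or below clamps health to zero, sets IsDead and returns it.
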(event `self.ReceiveBeginPlay`
  (`self.InitializeStat`))

(fn `DecreaseHealth`
  (params (DamagePoint :type "Float (double-precision)"))
  (returns (IsDead :type Boolean))
  (set `self.CurrentHealth` (- DamagePoint (`self.CurrentHealth`)))
  (if (<= (`self.CurrentHealth`) 0.0)
    (set `self.CurrentHealth` 0.0)
    (bind _output_get (set `self.IsDead` true))
    (return _output_get)))

(fn `IncreaseHealth`
  (params (HealthPoint :type "Float (double-precision)"))
  (set `self.CurrentHealth` (+ HealthPoint (`self.CurrentHealth`)))
  (if (> (`self.CurrentHealth`) (`self.MaxHealth`))
    (set `self.CurrentHealth` (`self.MaxHealth`))))

(fn `InitializeStat`
  (set `self.CurrentHealth` (`self.MaxHealth`)))