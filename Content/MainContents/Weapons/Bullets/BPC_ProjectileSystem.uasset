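; Actor component that simulates its owning bullet actor's flight and impacts, destroying it on hit or when its lifetime ends.
; Each tick it line-traces one velocity step, then moves the owner and adjusts vertical velocity using gravity and a speed-based drag term.
; Hits apply fixed damage to Enemy-tagged actors or spawn a bullet-hole decal otherwise.
; Data-table penetration and reverse-trace exit-point helpers are defined but unused in this flow.
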(event `self.ReceiveBeginPlay`
  (bind _returnvalue (`self.GetOwner`))
  (set `self.BulletVelocity` (* (`Actor.GetActorForwardVector` _returnvalue) (`self.BulletSpeed`)))
  (set `self.StartLocation` (`Actor.K2_GetActorLocation` _returnvalue))
  (set `self.CurrentWeapon` null)
  (set `self.IsBulletInitialize` true)
  (`KismetSystemLibrary.Delay` (`self.BulletLifeTime`))
  (`Actor.K2_DestroyActor` (`self.GetOwner`)))

(event `self.ReceiveTick`
  (params (DeltaSeconds :type "Float (single-precision)"))
  (if (`self.IsBulletInitialize`)
    (set `self.DeltaTime` DeltaSeconds)
    (set `self.StartLocation` (`Actor.K2_GetActorLocation` (`self.GetOwner`)))
    (set `self.NextLocation` (+ (`self.StartLocation`) (* (`self.BulletVelocity`) (`self.DeltaTime`))))
    (bind (_outhit _returnvalue) (`KismetSystemLibrary.LineTraceSingle` (`self.StartLocation`) (`self.NextLocation`) "TraceTypeQuery1" false (`|MakeArray` (`self.ActorToIgnore`)) "ForDuration" true (struct :`R` 1.0 :`A` 1.0) (struct :`G` 1.0 :`A` 1.0) 10.0))
    (if _returnvalue
      (bind (_bblockinghit _binitialoverlap _time _distance _location _impactpoint _normal _impactnormal _physmat _hitactor) (`GameplayStatics.BreakHitResult` _outhit))
      (if (`Actor.ActorHasTag` _hitactor "Enemy")
        (`GameplayStatics.ApplyDamage` _hitactor 20.0)
        (`Actor.K2_DestroyActor` (`self.GetOwner`))
        (else
          (set `self.OutHit` _outhit)
          (`self.CreateBulletHole` (struct))
          (`Actor.K2_DestroyActor` (`self.GetOwner`))))
      (else
        (`Actor.K2_SetActorLocation` (`self.GetOwner`) (`self.NextLocation`) false false)
        (set `self.BulletVelocity` (`self.CalculateGravityAndDecelaration` (`self.BulletVelocity`)))))))

(fn `CalculateExitBulletHoleLocation`
  (params (Direction :type "Vector Structure") (HitResult :type "HitResult Structure"))
  (returns (ExitLocation :type "Vector Structure") (SurfaceNormal :type "Vector Structure") (OutHit :type "HitResult Structure") (IsPenetrate :type Boolean))
  (locals (TraceDistance :type "Float (double-precision)") (TraceStartLocation :type "Vector Structure") (TraceEndLocation :type "Vector Structure") (ActorsToIgnore :type "Array of Actor Object Reference"))
  (bind (_bblockinghit _binitialoverlap _time _distance _location _impactpoint _normal _impactnormal _physmat _hitactor) (`GameplayStatics.BreakHitResult` HitResult))
  (bind (_origin _boxextent) (`Actor.GetActorBounds` _hitactor true true))
  (set `local.TraceDistance` (* (`KismetMathLibrary.FMax` (.x _boxextent) (.y _boxextent) (.z _boxextent)) 4.0))
  (bind _output_get (set `local.TraceStartLocation` (+ (* (`local.Direction`) (`local.TraceDistance`)) _impactpoint)))
  (set `local.TraceEndLocation` (+ _output_get (* (`local.Direction`) (* (`local.TraceDistance`) -1.0))))
  (bind (_outhit _returnvalue) (`KismetSystemLibrary.LineTraceSingle` (`local.TraceStartLocation`) (`local.TraceEndLocation`) "TraceTypeQuery1" false (`local.ActorsToIgnore`) :!label _label))
  (if _returnvalue
    (bind (_bblockinghit_2 _binitialoverlap_2 _time_2 _distance_2 _location_2 _impactpoint_2 _normal_2 _impactnormal_2 _physmat_2 _hitactor_2) (`GameplayStatics.BreakHitResult` _outhit))
    (if (!= _hitactor_2 _hitactor)
      (`KismetArrayLibrary.Array_Add` (`local.ActorsToIgnore`) _hitactor_2)
      (set `local.TraceStartLocation` _impactpoint_2)
      (goto _label)
      (else
        (return _impactpoint_2 _impactnormal_2 _outhit false)))
    (else
      (return (0.0 0.0 0.0) _impactnormal_2 (struct) false))))

(fn `CalculateGravityAndDecelaration`
  (params (Velocity :type "Vector Structure"))
  (returns (ReturnValue :type "Vector Structure"))
  (return (+ Velocity (* (`KismetMathLibrary.MakeVector` 0.0 0.0 (+ (`self.DragForce` (`self.AirDensity`) (`self.BulletSpeed`) (`self.CrossSection`) (`self.DragCoefficiency`)) (* (* (`self.Gravity`) 100.0) (`self.BulletMass`) -1.0))) (`self.DeltaTime`)))))

(fn `CanPenetrate`
  (params (BulletVelocity :type "Vector Structure") (HitResult :type "HitResult Structure"))
  (returns (ReturnValue :type Boolean))
  (bind _returnvalue (`|GetDataTableRow` "/Game/MainContents/Weapons/Bullets/DT_PenetrationData.DT_PenetrationData" (`KismetStringLibrary.Conv_StringToName` (`KismetSystemLibrary.GetObjectName` (`.PhysMat` (`GameplayStatics.BreakHitResult` HitResult)))))
    (:`then`
      (return (<= (`.MinVelocityToPenetrate_6_CEA44ABB43B9D6FC7FCC5ABA7CF2CE77` (break `/Game/MainContents/Weapons/Bullets/S_PenetrationData` _returnvalue)) (`KismetMathLibrary.VSize` (`local.BulletVelocity`)))))
    (:`RowNotFound`
      (return false))))

(fn `CreateBulletHole`
  (params (HitResult :type "HitResult Structure"))
  (bind (_bblockinghit _binitialoverlap _time _distance _location _impactpoint _normal _impactnormal) (`GameplayStatics.BreakHitResult` HitResult))
  (bind _returnvalue (`GameplayStatics.SpawnDecalAtLocation` "/Game/MainContents/Weapons/Bullets/M_BulletHole.M_BulletHole" (1.0 10.0 10.0) _location (`KismetMathLibrary.MakeRotFromX` _impactnormal)))
  (`DecalComponent.SetFadeScreenSize` _returnvalue 0.01))

(fn `DragForce`
  (params (AirDensity :type "Float (double-precision)") (BulletSpeed :type "Float (double-precision)") (CrossSection :type "Float (double-precision)") (DragCoefficiency :type "Float (double-precision)"))
  (returns (ReturnValue :type "Float (double-precision)"))
  ; 공기저항 함수
  (return (* (/ (* (* (* AirDensity (`KismetMathLibrary.Square` BulletSpeed)) CrossSection) DragCoefficiency) 2.0) -1.0)))