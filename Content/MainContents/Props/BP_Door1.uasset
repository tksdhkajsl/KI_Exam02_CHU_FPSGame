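; BP_Door1 is a door prop that opens when the first floor is cleared.
; BeginPlay caches the Door component's relative Z as the starting position.
; The ClearFloor1 event casts the player character to BP_Player and requires its KillCount to equal exactly nine.
; The OpenDoor timeline then offsets the door's relative Z from that start, scaled by MaxDoorLocation.
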(event `self.ReceiveBeginPlay`
  (bind (_relativelocation_x _relativelocation_y _relativelocation_z) (`KismetMathLibrary.BreakVector` (`SceneComponent.RelativeLocation` (`self.Door`))))
  (set `self.StartDoorLocation` _relativelocation_z))

(event `ClearFloor1`
  (bind _asbp_player (cast `/Game/MainContents/Charactor/Player/BP_Player` (`GameplayStatics.GetPlayerCharacter` 0)))
  (if (== (`/Game/MainContents/Charactor/Player/BP_Player.KillCount` _asbp_player) 9)
    (bind (_direction _opendoor) (`Timeline|OpenDoor`)
      (:`Update`
        (`SceneComponent.K2_SetRelativeLocation` (`self.Door`) (`KismetMathLibrary.MakeVector` 0.0 0.0 (+ (`self.StartDoorLocation`) (* _opendoor (`self.MaxDoorLocation`) 1.0))) false false)))))

(fn `UserConstructionScript`)