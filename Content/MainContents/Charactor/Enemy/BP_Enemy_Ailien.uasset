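; Alien enemy character that chases and melees the player, driven by AIC_Enemy and its blackboard.
; A detector overlap hands the player to the controller as target, while StartAttack sets a timer for a right-arm sphere trace that damages the player.
; Damage feeds BPCStatSystem and sets hit or death blackboard flags with matching montages.
; Death increments the player's kill count, calls EndGame and door-clear functions, then destroys the actor after a delay.
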(event `self.ReceiveBeginPlay`
  ; Initialize(초기화) IDLE 실행
  (bind _asabp_enemy_ailien (cast `/Game/MainContents/Charactor/Enemy/ABP_Enemy_Ailien` (`SkeletalMeshComponent.GetAnimInstance` (`self.Mesh`))))
  (set `self.AnimationBP` _asabp_enemy_ailien)
  (set `/Game/MainContents/Charactor/BPC_StatSystem.CurrentHealth` 100.0 (`self.BPC_StatSystem`)))

(event `self.ReceiveAnyDamage`
  (params (Damage :type "Float (single-precision)") (DamageType :type "DamageType Object Reference") (InstigatedBy :type "Controller Object Reference") (DamageCauser :type "Actor Object Reference"))
  ; 공격 받은 후 처리 이벤트
  (bind _output_get (set `self.IsHit` true))
  (`BlackboardComponent.SetValueAsBool` (`AIBlueprintHelperLibrary.GetBlackboard` null) (`self.IsHitBlackboardKey`) _output_get)
  (bind _isdead (`/Game/MainContents/Charactor/BPC_StatSystem.DecreaseHealth` (`self.BPC_StatSystem`) Damage null))
  (bind _output_get_2 (set `self.IsDead` _isdead))
  (if _output_get_2
    (`PrimitiveComponent.SetCollisionEnabled` (`self.CapsuleComponent`) "NoCollision")
    (`PrimitiveComponent.SetCollisionEnabled` (`self.Mesh`) "NoCollision")
    (bind _asbp_player (cast `/Game/MainContents/Charactor/Player/BP_Player` (`GameplayStatics.GetPlayerCharacter` 0)))
    (set `/Game/MainContents/Charactor/Player/BP_Player.KillCount` (+ (`/Game/MainContents/Charactor/Player/BP_Player.KillCount` _asbp_player) 1) _asbp_player)
    (`BlackboardComponent.SetValueAsBool` (`AIBlueprintHelperLibrary.GetBlackboard` null) (`self.IsDeadBlackboardKey`) (`self.IsDead`))
    (`self.PlayAnimMontage` "/Game/MainContents/Animation/Enemy/Montage/Ailien_Death_Anim_Montage.Ailien_Death_Anim_Montage")
    (`|ExecutionSequence`
      (:`then_0`
        (`/Game/MainContents/Charactor/Player/BP_Player.EndGame` _asbp_player)
        (`/Game/MainContents/Props/BP_Door1.ClearFloor1` (`self.Door1`))
        (`/Game/MainContents/Props/BP_Door2.ClearFloor2` (`self.Door2`)))
      (:`then_1`
        (`KismetSystemLibrary.Delay` (`self.Duration`))
        (`self.K2_DestroyActor`)))
    (else
      (bind _returnvalue (`self.PlayAnimMontage` "/Game/MainContents/Animation/Enemy/Montage/Ailien_Reaction_Hit_Montage.Ailien_Reaction_Hit_Montage"))
      (`KismetSystemLibrary.Delay` _returnvalue)
      (bind _output_get_3 (set `self.IsHit` false))
      (`BlackboardComponent.SetValueAsBool` (`AIBlueprintHelperLibrary.GetBlackboard` null) (`self.IsHitBlackboardKey`) _output_get_3))))

(event `self.TempDetector.OnComponentBeginOverlap`
  (params (OverlappedComponent :type "PrimitiveComponent Object Reference") (OtherActor :type "Actor Object Reference") (OtherComp :type "PrimitiveComponent Object Reference") (OtherBodyIndex :type Integer) (bFromSweep :type Boolean) (SweepResult :type "HitResult Structure (by ref)"))
  ; 시야 범위 침입 시  추적
  (bind _asbp_player (cast `/Game/MainContents/Charactor/Player/BP_Player` OtherActor))
  (bind _asaic_enemy (cast `/Game/MainContents/Charactor/Enemy/AIC_Enemy` (`AIBlueprintHelperLibrary.GetAIController` self)))
  (`/Game/MainContents/Charactor/Enemy/AIC_Enemy.SetTarget` _asaic_enemy _asbp_player))

(event `StartAttack`
  (bind _returnvalue (`KismetSystemLibrary.K2_SetTimerDelegate` (delegate `Attack`) 0.01))
  (set `self.AttackTimerHandler` _returnvalue))

(event `Attack`
  (bind (_outhit _returnvalue) (`KismetSystemLibrary.SphereTraceSingle` (`SceneComponent.K2_GetComponentLocation` (`self.RightArmStart`)) (`SceneComponent.K2_GetComponentLocation` (`self.RightArmEnd`)) 30.0 "TraceTypeQuery1"))
  (if _returnvalue
    (bind (_bblockinghit _binitialoverlap _time _distance _location _impactpoint _normal _impactnormal _physmat _hitactor) (`GameplayStatics.BreakHitResult` _outhit))
    (if (`self.ActorHasTag` _hitactor "Player")
      (`GameplayStatics.ApplyDamage` _hitactor 20.0 null self))))

(event `StopAttack`
  (`KismetSystemLibrary.K2_ClearAndInvalidateTimerHandle` (`self.AttackTimerHandler`)))

(fn `InitializeStat`
  (params (PlayerHUD :type "/Game/MainContents/UI/WBP_Player Object Reference")))

(fn `UserConstructionScript`)