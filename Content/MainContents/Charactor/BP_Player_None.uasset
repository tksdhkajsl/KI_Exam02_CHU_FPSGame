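; Player character Blueprint that handles movement, mouse look and switching between third-person and first-person cameras through Enhanced Input.
; On BeginPlay it caches the BP_PlayerControl controller, adds IMC_Player and starts on the third-person view.
; Movement follows the actor's facing, and look input drives controller yaw and pitch.
; A FlipFlop toggles IsTPSMode and blends the view target between two child-actor cameras.
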(event `self.ReceiveBeginPlay`
  ; Initialize
  (bind _asbp_player_control (cast `/Game/MainContents/Control/BP_PlayerControl` (`self.GetController`)))
  (bind _output_get (set `self.PlayerController` _asbp_player_control))
  (`EnhancedInputSubsystemInterface.AddMappingContext` (pcsubsystem `EnhancedInputLocalPlayerSubsystem` _output_get) "/Game/MainContents/Control/Input/IMC_Player.IMC_Player" 0 (struct))
  (`PlayerController.SetViewTargetWithBlend` (`self.PlayerController`) (`ChildActorComponent.ChildActor` (`self.TPSCamera`)) 0.0 "VTBlend_Linear" 0.0 false))

(event `EnhancedInput|/Game/MainContents/Control/Input/IA_Movement`
  (params (ActionValue :type "Vector2D Structure") (ElapsedSeconds :type "Float (double-precision)") (TriggeredSeconds :type "Float (double-precision)") (InputAction :type "InputAction Object Reference" :default "/Game/MainContents/Control/Input/IA_Movement.IA_Movement"))
  (bind (_returnvalue_roll _returnvalue_pitch _returnvalue_yaw) (`KismetMathLibrary.BreakRotator` (`self.K2_GetActorRotation`)))
  (bind (_returnvalue_roll_2 _returnvalue_pitch_2 _returnvalue_yaw_2) (`KismetMathLibrary.BreakRotator` (`self.K2_GetActorRotation`)))
  ; Moving
  (:`Triggered`
    (`self.AddMovementInput` (`KismetMathLibrary.GetRightVector` (`KismetMathLibrary.MakeRotator` _returnvalue_roll 0.0 _returnvalue_yaw)) ActionValue_X)
    (`self.AddMovementInput` (`KismetMathLibrary.GetForwardVector` (`KismetMathLibrary.MakeRotator` 0.0 0.0 _returnvalue_yaw_2)) ActionValue_Y)))

(event `EnhancedInput|/Game/MainContents/Control/Input/IA_CameraMode`
  (params (ActionValue :type Boolean) (ElapsedSeconds :type "Float (double-precision)") (TriggeredSeconds :type "Float (double-precision)") (InputAction :type "InputAction Object Reference" :default "/Game/MainContents/Control/Input/IA_CameraMode.IA_CameraMode"))
  (:`Started`
    (`/Engine/EditorBlueprintResources/StandardMacros.FlipFlop`
      (:`A`
        (set `self.IsTPSMode` false)
        (`PlayerController.SetViewTargetWithBlend` (`self.PlayerController`) (`ChildActorComponent.ChildActor` (`self.FPSCamera`)) (`self.CameraBlendTime`) "VTBlend_Linear" 0.0 false)
        (`KismetSystemLibrary.Delay` (`self.CameraBlendTime`)))
      (:`B`
        (set `self.IsTPSMode` true)
        (`PlayerController.SetViewTargetWithBlend` (`self.PlayerController`) (`ChildActorComponent.ChildActor` (`self.TPSCamera`)) (`self.CameraBlendTime`) "VTBlend_Linear" 0.0 false)))))

(event `EnhancedInput|/Game/MainContents/Control/Input/IA_LookAround`
  (params (ActionValue :type "Vector2D Structure") (ElapsedSeconds :type "Float (double-precision)") (TriggeredSeconds :type "Float (double-precision)") (InputAction :type "InputAction Object Reference" :default "/Game/MainContents/Control/Input/IA_LookAround.IA_LookAround"))
  ; 마우스 시점
  (:`Triggered`
    (`self.AddControllerYawInput` ActionValue_X)
    (`self.AddControllerPitchInput` ActionValue_Y)))

(fn `UserConstructionScript`)