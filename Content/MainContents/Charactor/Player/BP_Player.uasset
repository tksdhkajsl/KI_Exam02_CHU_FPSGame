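; Player character Blueprint for a TPS/FPS shooter, handling Enhanced Input movement, jump, lean, view switching and zoom by blending between child-actor cameras.
; Picked-up weapons attach to type-specific sockets and drop the previous one.
; Pistols and assault rifles fire manually or on a looping timer, spawning bullets with recoil and debug traces.
; BPCStatSystem resolves damage, death reloads the map, and reaching the kill count shows the clear widget.
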(event `EnhancedInput|/Game/MainContents/Control/Input/IA_PickUp`
  (params (ActionValue :type Boolean) (ElapsedSeconds :type "Float (double-precision)") (TriggeredSeconds :type "Float (double-precision)") (InputAction :type "InputAction Object Reference" :default "/Game/MainContents/Control/Input/IA_PickUp.IA_PickUp"))
  ; 무기 픽업 이벤트
  (:`Started`
    (message `/Game/MainContents/Interfaces/BPI_Interact.PickUp` (`|GetArrayItem` (`self.GetOverlappingActors` "/Game/MainContents/Weapons/BP_PickUpWeaponMaster.BP_PickUpWeaponMaster_C")) self)))

(event `self.ReceiveBeginPlay`
  ; Initialize
  (bind _asbp_player_control (cast `/Game/MainContents/Control/BP_PlayerControl` (`self.GetController`)))
  (bind _output_get (set `self.PlayerController` _asbp_player_control))
  (`EnhancedInputSubsystemInterface.AddMappingContext` (pcsubsystem `EnhancedInputLocalPlayerSubsystem` _output_get) "/Game/MainContents/Control/Input/IMC_Player.IMC_Player" 0 (struct))
  (`PlayerController.SetViewTargetWithBlend` (`self.PlayerController`) (`ChildActorComponent.ChildActor` (`self.TPSCamera`)) 0.0 "VTBlend_Linear" 0.0 false)
  (set `self.IsTPSMode` true))

(event `PickUpWeapon`
  (params (EquipWeapon :type "/Game/MainContents/Weapons/BP_EquipWeaponMaster Class Reference"))
  (bind _currentweapon (`self.CurrentWeapon`))
  ; 신규 무기 픽업 후 기존 무기 소멸이 아닌 땅바닥에 버려지고, 신규무기 장착
  (`/Engine/EditorBlueprintResources/StandardMacros.IsValid` _currentweapon
    (:`Is Valid`
      (`|SpawnActorFromClass` (`/Game/MainContents/Weapons/BP_EquipWeaponMaster.Pickup Weapon` _currentweapon) (`KismetMathLibrary.MakeTransform` (+ (`self.K2_GetActorLocation`) (* (`self.GetActorForwardVector`) (50.0 50.0 0.0)))) "Undefined" "MultiplyWithRoot" null null)
      (`self.K2_DestroyActor` _currentweapon))
    (:`Is Not Valid`
      _))
  (bind _returnvalue (`|SpawnActorFromClass` EquipWeapon (`KismetMathLibrary.MakeTransform` (0.0 0.0 0.0)) "Undefined" "MultiplyWithRoot" null null))
  (`self.PickUpWeaponType` _returnvalue))

(event `EnhancedInput|/Game/MainContents/Control/Input/IA_Movement`
  (params (ActionValue :type "Vector2D Structure") (ElapsedSeconds :type "Float (double-precision)") (TriggeredSeconds :type "Float (double-precision)") (InputAction :type "InputAction Object Reference" :default "/Game/MainContents/Control/Input/IA_Movement.IA_Movement"))
  (bind (_returnvalue_roll _returnvalue_pitch _returnvalue_yaw) (`KismetMathLibrary.BreakRotator` (`self.GetControlRotation`)))
  (bind (_returnvalue_roll_2 _returnvalue_pitch_2 _returnvalue_yaw_2) (`KismetMathLibrary.BreakRotator` (`self.GetControlRotation`)))
  ; Moving
  (:`Triggered`
    (`self.AddMovementInput` (`KismetMathLibrary.GetRightVector` (`KismetMathLibrary.MakeRotator` _returnvalue_roll_2 0.0 _returnvalue_yaw_2)) ActionValue_X)
    (`self.AddMovementInput` (`KismetMathLibrary.GetForwardVector` (`KismetMathLibrary.MakeRotator` 0.0 0.0 _returnvalue_yaw)) ActionValue_Y)))

(event `EnhancedInput|/Game/MainContents/Control/Input/IA_Fire`
  (params (ActionValue :type Boolean) (ElapsedSeconds :type "Float (double-precision)") (TriggeredSeconds :type "Float (double-precision)") (InputAction :type "InputAction Object Reference" :default "/Game/MainContents/Control/Input/IA_Fire.IA_Fire"))
  ; 총기 발사 및 반동
  (:`Started`
    (set `self.IsFiring` true)
    (bind _currentweapon (`self.CurrentWeapon`)
      (:`then`
        (switch `/Game/MainContents/Weapons/E_WeaponType` (`/Game/MainContents/Weapons/BP_EquipWeaponMaster.Weapon Type` _currentweapon)
          (:`NewEnumerator0`
            _)
          (:`NewEnumerator1`
            _))
        (switch `/Game/MainContents/Weapons/E_FireMode` (`/Game/MainContents/Weapons/BP_EquipWeaponMaster.FireMode` _currentweapon)
          (:`NewEnumerator0`
            (`self.FireBullet`)
            (`self.GunRebound`)
            (`self.LineTrace`))
          (:`NewEnumerator1`
            (`self.FireBullet`)
            (`self.GunRebound`)
            (bind _returnvalue (`KismetSystemLibrary.K2_SetTimerDelegate` (delegate `Onfire`) (`/Game/MainContents/Weapons/BP_EquipWeaponMaster.FireRate` (`self.CurrentWeapon`)) true))
            (set `self.TimerHandler` _returnvalue))))
      (:`else`)))
  (:`Canceled`
    (set `self.IsFiring` false :!label _label)
    (message `/Game/MainContents/Interfaces/BPI_Fire.Fire` (`SkeletalMeshComponent.GetAnimInstance` (`self.Mesh`)) (`self.IsFiring`))
    (`KismetSystemLibrary.K2_ClearAndInvalidateTimerHandle` (`self.TimerHandler`)))
  (:`Completed`
    (goto _label)))

(event `EnhancedInput|/Game/MainContents/Control/Input/IA_LookAround`
  (params (ActionValue :type "Vector2D Structure") (ElapsedSeconds :type "Float (double-precision)") (TriggeredSeconds :type "Float (double-precision)") (InputAction :type "InputAction Object Reference" :default "/Game/MainContents/Control/Input/IA_LookAround.IA_LookAround"))
  ; 마우스 시점
  (:`Triggered`
    (`self.AddControllerYawInput` ActionValue_X)
    (`self.AddControllerPitchInput` ActionValue_Y)
    (set `self.Pitch` (`KismetMathLibrary.FClamp` (+ ActionValue_Y (`self.Pitch`)) (`self.Min`) (`self.Max`)))))

(event `Onfire`
  ; 총기 발사 및 반동
  (`self.FireBullet`)
  (`self.GunRebound`)
  (`self.LineTrace`))

(event `EnhancedInput|/Game/MainContents/Control/Input/IA_Leaning`
  (params (ActionValue :type "Float (double-precision)") (ElapsedSeconds :type "Float (double-precision)") (TriggeredSeconds :type "Float (double-precision)") (InputAction :type "InputAction Object Reference" :default "/Game/MainContents/Control/Input/IA_Leaning.IA_Leaning"))
  ; 몸통 좌우 움직이기
  (:`Triggered`
    (if (not (`self.IsJumping`))
      (set `self.IsLeaning` false)
      (set `self.Roll` (`KismetMathLibrary.FInterpTo` (`self.Roll`) (`KismetMathLibrary.MapRangeClamped` ActionValue -1.0 1.0 -10.0 10.0) (`GameplayStatics.GetWorldDeltaSeconds`) 5.0))))
  (:`Canceled`
    (if (not (`self.IsJumping`)) :!label _label_2
      (bind _output_get (set `self.IsLeaning` true))
      (if (and _output_get (!= (`self.Roll`) 0.0)) :!label _label_3
        (set `self.Roll` (`KismetMathLibrary.FInterpTo` (`self.Roll`) 0.0 (`GameplayStatics.GetWorldDeltaSeconds`) 5.0))
        (goto _label_3)
        (else
          (set `self.IsLeaning` false)))))
  (:`Completed`
    (goto _label_2)))

(event `SpawnBullet`
  ; 총알 생성
  (`|SpawnActorFromClass` "/Game/MainContents/Weapons/Bullets/BP_Bullet.BP_Bullet_C" (`SceneComponent.GetSocketTransform` (`/Game/MainContents/Weapons/BP_EquipWeaponMaster.Weapon` (`self.CurrentWeapon`)) "Muzzle" "RTS_World") "Undefined" "MultiplyWithRoot" null null))

(event `LineTrace`
  (bind _weapon (`/Game/MainContents/Weapons/BP_EquipWeaponMaster.Weapon` (`self.CurrentWeapon`)))
  (bind _returnvalue (`SceneComponent.GetSocketLocation` _weapon "Muzzle"))
  ; LineTrace(테스트용 총알 낙차 및 방향 확인용)
  (bind (_outhit _returnvalue_2) (`KismetSystemLibrary.LineTraceSingle` _returnvalue (+ _returnvalue (* (`KismetMathLibrary.GetForwardVector` (`SceneComponent.GetSocketRotation` _weapon "Muzzle")) 10000.0)) "TraceTypeQuery1" false (`|MakeArray` (`self.CurrentWeapon`) :!type "Actor Object Reference") "ForDuration" true (struct :`R` 1.0 :`A` 1.0) (struct :`G` 1.0 :`A` 1.0) 0.5))
  (if _returnvalue_2
    (`|SpawnActorFromClass` "/Game/MainContents/Weapons/BP_ImpactField.BP_ImpactField_C" (`KismetMathLibrary.MakeTransform` (`.ImpactPoint` (`GameplayStatics.BreakHitResult` _outhit))) "Undefined" "MultiplyWithRoot" null null)))

(event `EnhancedInput|/Game/MainContents/Control/Input/IA_Change`
  (params (ActionValue :type Boolean) (ElapsedSeconds :type "Float (double-precision)") (TriggeredSeconds :type "Float (double-precision)") (InputAction :type "InputAction Object Reference" :default "/Game/MainContents/Control/Input/IA_Change.IA_Change"))
  (bind _currentweapon (`self.CurrentWeapon`))
  ; 총기 단발/연사 변경
  (:`Started`
    (bind _currentweapon_2 (`self.CurrentWeapon`)
      (:`then`
        (switch `/Game/MainContents/Weapons/E_FireMode` (`/Game/MainContents/Weapons/BP_EquipWeaponMaster.FireMode` _currentweapon_2)
          (:`NewEnumerator0`
            (message `/Game/MainContents/Interfaces/BPI_EquipWeaponInterface.SetFireMode` _currentweapon "NewEnumerator1")
            (`KismetSystemLibrary.PrintString` "Auto"))
          (:`NewEnumerator1`
            (message `/Game/MainContents/Interfaces/BPI_EquipWeaponInterface.SetFireMode` _currentweapon "NewEnumerator0")
            (`KismetSystemLibrary.PrintString` "Manual"))))
      (:`else`))))

(event `EnhancedInput|/Game/MainContents/Control/Input/IA_Jumping`
  (params (ActionValue :type Boolean) (ElapsedSeconds :type "Float (double-precision)") (TriggeredSeconds :type "Float (double-precision)") (InputAction :type "InputAction Object Reference" :default "/Game/MainContents/Control/Input/IA_Jumping.IA_Jumping"))
  ; 점프
  (:`Started`
    (set `self.IsJumping` true)
    (`self.Jump`))
  (:`Canceled`
    (set `self.IsJumping` false :!label _label_4)
    (`self.StopJumping`))
  (:`Completed`
    (goto _label_4)))

(event `EnhancedInput|/Game/MainContents/Control/Input/IA_CameraMode`
  (params (ActionValue :type Boolean) (ElapsedSeconds :type "Float (double-precision)") (TriggeredSeconds :type "Float (double-precision)") (InputAction :type "InputAction Object Reference" :default "/Game/MainContents/Control/Input/IA_CameraMode.IA_CameraMode"))
  ; 카메라 시점 변환
  (:`Started`
    (`/Engine/EditorBlueprintResources/StandardMacros.FlipFlop`
      (:`A`
        (set `self.IsTPSMode` false)
        (`PlayerController.SetViewTargetWithBlend` (`self.PlayerController`) (`ChildActorComponent.ChildActor` (`self.FPSCamera`)) (`self.CameraBlendTime`) "VTBlend_Linear" 0.0 false)
        (`KismetSystemLibrary.Delay` (`self.CameraBlendTime`))
        (`SceneComponent.SetHiddenInGame` (`self.Helmet`) true true))
      (:`B`
        (set `self.IsTPSMode` true)
        (`PlayerController.SetViewTargetWithBlend` (`self.PlayerController`) (`ChildActorComponent.ChildActor` (`self.TPSCamera`)) (`self.CameraBlendTime`) "VTBlend_Linear" 0.0 false)
        (`SceneComponent.SetHiddenInGame` (`self.Helmet`) false true)))))

(event `EnhancedInput|/Game/MainContents/Control/Input/IA_Zoom`
  (params (ActionValue :type Boolean) (ElapsedSeconds :type "Float (double-precision)") (TriggeredSeconds :type "Float (double-precision)") (InputAction :type "InputAction Object Reference" :default "/Game/MainContents/Control/Input/IA_Zoom.IA_Zoom"))
  (bind _camerablendtime (`self.CameraBlendTime`))
  (bind _camerablendtime_2 (`self.CameraBlendTime`))
  (bind _currentweapon (`self.CurrentWeapon`))
  ; 줌인/아웃
  (:`Started`
    (if (`self.IsTPSMode`)
      (`PlayerController.SetViewTargetWithBlend` (`self.PlayerController`) (`ChildActorComponent.ChildActor` (`self.TPSZoomCamera`)) _camerablendtime_2 "VTBlend_Linear" 0.0 false)
      (else
        (`/Engine/EditorBlueprintResources/StandardMacros.IsValid` _currentweapon
          (:`Is Valid`
            (`PlayerController.SetViewTargetWithBlend` (`self.PlayerController`) (`ChildActorComponent.ChildActor` (`/Game/MainContents/Weapons/BP_EquipWeaponMaster.ChildActor` _currentweapon)) _camerablendtime_2 "VTBlend_Linear" 0.0 false)))))
    (set `self.IsZoomed` true))
  (:`Canceled`
    (if (`self.IsTPSMode`) :!label _label_5
      (`PlayerController.SetViewTargetWithBlend` (`self.PlayerController`) (`ChildActorComponent.ChildActor` (`self.TPSCamera`)) _camerablendtime "VTBlend_Linear" 0.0 false)
      (set `self.IsZoomed` false)
      (else
        (`PlayerController.SetViewTargetWithBlend` (`self.PlayerController`) (`ChildActorComponent.ChildActor` (`self.FPSCamera`)) _camerablendtime "VTBlend_Linear" 0.0 false))))
  (:`Completed`
    (goto _label_5)))

(event `self.ReceiveAnyDamage`
  (params (Damage :type "Float (single-precision)") (DamageType :type "DamageType Object Reference") (InstigatedBy :type "Controller Object Reference") (DamageCauser :type "Actor Object Reference"))
  (set `self.IsHiting` true)
  (bind _isdead (`/Game/MainContents/Charactor/BPC_StatSystem.DecreaseHealth` (`self.BPC_StatSystem`) Damage (`/Game/MainContents/Control/BP_PlayerControl.PlayerHUD` (`self.PlayerController`))))
  (bind _output_get (set `self.IsDead` _isdead))
  (if _output_get
    (`self.PlayAnimMontage` "/Game/MainContents/Animation/Player/Player_Death_Anim_Montage.Player_Death_Anim_Montage")
    (`KismetSystemLibrary.Delay` 1.0)
    (bind (_outactor _returnvalue) (`LevelSequencePlayer.CreateLevelSequencePlayer` "/Game/MainContents/Map/Fade.Fade"))
    (`MovieSceneSequencePlayer.Play` _returnvalue)
    (`KismetSystemLibrary.Delay` 3.0)
    (`GameplayStatics.OpenLevel` "TfirdPersonMap")
    (else
      (`self.PlayAnimMontage` "/Game/MainContents/Animation/Player/Re_Hit_Reaction__1__Anim_Montage.Re_Hit_Reaction__1__Anim_Montage")
      (set `self.IsHiting` false))))

(event `EndGame`
  (if (== (`self.TotalKill`) (`self.KillCount`))
    (`/Engine/EditorBlueprintResources/StandardMacros.DoOnce` false
      (:`Completed`
        (bind (_outactor _returnvalue) (`LevelSequencePlayer.CreateLevelSequencePlayer` "/Game/MainContents/Map/Dark.Dark"))
        (`MovieSceneSequencePlayer.Play` _returnvalue)
        (`KismetSystemLibrary.Delay` 2.0)
        (bind _returnvalue_2 (`|CreateWidget` "/Game/MainContents/UI/WBP_ClearOption.WBP_ClearOption_C" (`GameplayStatics.GetPlayerController` 0)))
        (bind _output_get (set `self.Widget` _returnvalue_2))
        (`UserWidget.AddToViewport` _output_get 0)))))

(fn `FireBullet`
  (message `/Game/MainContents/Interfaces/BPI_Fire.Fire` (`SkeletalMeshComponent.GetAnimInstance` (`self.Mesh`)) (`self.IsFiring`))
  (`self.SpawnBullet`)
  (`/Game/MainContents/Interfaces/BPI_Fire.Fire` (`self.CurrentWeapon`) false))

(fn `GunRebound`
  (`self.AddControllerYawInput` -1.0)
  (set `self.Pitch` (+ (`self.Pitch`) -1.0)))

(fn `PickUpWeaponType`
  (params (CurrentWeapon :type "/Game/MainContents/Weapons/BP_EquipWeaponMaster Object Reference"))
  (bind _mesh (`self.Mesh`))
  (bind _output_get (set `self.CurrentWeapon` CurrentWeapon))
  (switch `/Game/MainContents/Weapons/E_WeaponType` (`/Game/MainContents/Weapons/BP_EquipWeaponMaster.Weapon Type` _output_get)
    (:`NewEnumerator0`
      (bind _returnvalue (`self.K2_AttachToComponent` _output_get _mesh "Pistol" "KeepRelative" "KeepRelative" "KeepRelative" true))
      (if _returnvalue
        (set `self.PlayerWeaponType` "NewEnumerator0")))
    (:`NewEnumerator1`
      (bind _returnvalue_2 (`self.K2_AttachToComponent` _output_get _mesh "AssaultRifle" "KeepRelative" "KeepRelative" "KeepRelative" true))
      (if _returnvalue_2
        (set `self.PlayerWeaponType` "NewEnumerator1")))
    (:`NewEnumerator2`
      (bind _returnvalue_3 (`self.K2_AttachToComponent` _output_get _mesh "SniperRifle" "KeepRelative" "KeepRelative" "KeepRelative" true))
      (if _returnvalue_3
        (set `self.PlayerWeaponType` "NewEnumerator2")))
    (:`NewEnumerator3`
      (bind _returnvalue_4 (`self.K2_AttachToComponent` _output_get _mesh "ShotGun" "KeepRelative" "KeepRelative" "KeepRelative" true))
      (if _returnvalue_4
        (set `self.PlayerWeaponType` "NewEnumerator3")))))

(fn `UserConstructionScript`
  (`parent.UserConstructionScript`)
  (`SkinnedMeshComponent.SetLeaderPoseComponent` (`self.Hands`) (`self.Mesh`) false false)
  (`SkinnedMeshComponent.SetLeaderPoseComponent` (`self.Legs_1`) (`self.Mesh`) false false)
  (`SkinnedMeshComponent.SetLeaderPoseComponent` (`self.Helmet`) (`self.Mesh`) false false)
  (`SkinnedMeshComponent.SetLeaderPoseComponent` (`self.Boots`) (`self.Mesh`) false false)
  (`SkinnedMeshComponent.SetLeaderPoseComponent` (`self.Armor`) (`self.Mesh`) false false)
  (`SkinnedMeshComponent.SetLeaderPoseComponent` (`self.Legs_2`) (`self.Mesh`) false false))